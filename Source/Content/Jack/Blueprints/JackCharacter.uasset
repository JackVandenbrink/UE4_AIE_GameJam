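; Jack's flipbook-sprite character, tethered to another character (OtherChar) and swinging from it like a rope.
; Each tick, when lower, or level without Priority, it corrects overstretch by blending toward mirrored velocity and pulling itself inward, recording blocking hits.
; Tick also drives idle, run, fall and land animations, sprite facing, and a kill-height Retry on the game instance.
; Gravity and jump velocity come from DesignerVariables; Lock stops ticking, and Died pins position while locked.
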(event `self.ReceiveBeginPlay`
  (`self.SpawnDefaultController`)
  (`self.Init`))

(event `Died`
  (`Timeline|Timeline_0` :!label _label
    (:`Update`
      (if (`self.Locked`)
        (set `MovementComponent.Velocity` (0.0 0.0 0.0) (`self.CharacterMovement`))
        (`self.K2_SetActorLocation` (`self.Pos`))
        (else
          (goto _label :!via `Stop`))))))

(event `self.ReceiveTick`
  (params (DeltaSeconds :type "Float (single-precision)"))
  (`self.SwingFromOther`)
  (`self.KillZ`)
  (`self.DetectLand`)
  (`self.IdleOrRunTick`)
  (`self.Flip`))

(event `Jumped`
  (params (IsOnGround :type Boolean))
  ;[1 1 1] Play jumping animation
  (if IsOnGround
    (set `self.Jump` true)
    (bind _time (`self.ChangeAnimation` "NewEnumerator2"))
    (`KismetSystemLibrary.Delay` _time)
    (set `self.Jump` false)))

(event `Landed`
  ;[1 1 1] Play landing animations
  (set `self.Land` true)
  (bind _time (`self.ChangeAnimation` "NewEnumerator4"))
  (`KismetSystemLibrary.Delay` _time)
  (set `self.Land` false))

(event `IdleOrRunTick`
  ;[0 1 0.793] Animation Detection VERY DELICATE
  (if (`NavMovementComponent.IsFalling` (`self.CharacterMovement`))
    (if (`self.Jump`)
      _
      (elif (not (`self.Falling`))
        (`self.ChangeAnimation` "NewEnumerator1")
        (set `self.Falling` true)
        (set `self.Idle` false)
        (set `self.Running` false)))
    (elif (`self.Land`)
      _
      (elif (== (`self.GetLastMovementInputVector`) (0.0 0.0 0.0))
        (if (not (`self.Idle`))
          (`self.ChangeAnimation` "NewEnumerator0")
          (set `self.Idle` true)
          (set `self.Running` false))
        (elif (not (`self.Running`))
          (`self.ChangeAnimation` "NewEnumerator3")
          (set `self.Running` true)
          (set `self.Idle` false))))))

(fn `ChangeAnimation`
  (params (NewAnimation :type "/Game/Jack/Blueprints/Anims/Animations Enum"))
  (returns (Time :type "Float (double-precision)"))
  (for _array_element (`self.Animations`)
    (if (`|EnumEquality` NewAnimation (break `/Game/Jack/Blueprints/Anims/AnimationsStructure` _array_element))
      (`PaperFlipbookComponent.SetFlipbook` (`self.Sprite`) (`.Flipbook_5_E831D69243C36909A4B819A579AA7B34` (break `/Game/Jack/Blueprints/Anims/AnimationsStructure` _array_element)))
      (return (`PaperFlipbook.GetTotalDuration` (`.Flipbook_5_E831D69243C36909A4B819A579AA7B34` (break `/Game/Jack/Blueprints/Anims/AnimationsStructure` _array_element)))))))

(fn `DetectLand`
  (if (`NavMovementComponent.IsFalling` (`self.CharacterMovement`))
    _
    (elif (`self.Falling`)
      (`self.Landed`)
      (set `self.Falling` false)))
  (return))

(fn `Flip`
  (bind (_returnvalue_x _returnvalue_y) (`KismetMathLibrary.BreakVector` (`self.GetLastMovementInputVector`)))
  (bind _sprite (`self.Sprite`))
  (if (>= _returnvalue_y 0.8)
    (`SceneComponent.K2_SetRelativeRotation` _sprite (`self.RunningRight`) false false)
    (elif (<= _returnvalue_y -0.8)
      (`SceneComponent.K2_SetRelativeRotation` _sprite (`self.RunningLeft`) false false))))

(fn `Init`
  (bind _charactermovement (`self.CharacterMovement`))
  (bind _asdesigner_variables (cast `/Game/DesignerVariables` (`GameplayStatics.GetGameState`)))
  (set `CharacterMovementComponent.GravityScale` (`/Game/DesignerVariables.GravityScale` _asdesigner_variables) _charactermovement)
  (set `CharacterMovementComponent.JumpZVelocity` (`/Game/DesignerVariables.JumpVelocity` _asdesigner_variables) _charactermovement))

(fn `IsOnGround`
  (returns (Return :type Boolean))
  (return (`NavMovementComponent.IsMovingOnGround` (`self.CharacterMovement`))))

(fn `KillZ`
  (if (<= (.z (`self.K2_GetActorLocation`)) (`self.KillZoneZ`))
    (bind _asgame_jam_instance (cast `/Game/GameJamInstance` (`GameplayStatics.GetGameInstance`)))
    (`/Game/GameJamInstance.Retry` _asgame_jam_instance)))

(fn `Lock`
  (params (NewLock :type Boolean))
  (bind _output_get (set `self.Locked` NewLock))
  (if _output_get
    (set `self.Pos` (`self.K2_GetActorLocation`))
    (`self.SetActorTickEnabled` false)
    (else
      (`self.SetActorTickEnabled` true))))

(fn `OtherIsBlocked`
  (returns (Return :type Boolean))
  (return (`/Game/Jack/Blueprints/JackCharacter.Blocked` (`self.OtherChar`))))

(fn `SwingFromOther`
  (bind _returnvalue (`self.K2_GetActorLocation`))
  (bind _maxdistance (`self.MaxDistance`))
  (bind _returnvalue_2 (`self.K2_GetActorLocation` (`self.OtherChar`)))
  (bind _returnvalue_3 (`KismetMathLibrary.FFloor` (.z (`self.K2_GetActorLocation` self))))
  (bind _returnvalue_4 (`KismetMathLibrary.FFloor` (.z (`self.K2_GetActorLocation` (`self.OtherChar`)))))
  (bind _returnvalue_5 (`KismetMathLibrary.VSize` (- _returnvalue_2 _returnvalue)))
  (if (>= (`KismetMathLibrary.Abs_Int` (- _returnvalue_3 _returnvalue_4)) 3)
    (if (< _returnvalue_3 _returnvalue_4)
      (if (> _returnvalue_5 _maxdistance) :!label _label
        ;[1 1 1] Set Velocity and Force Player Pos Inwards
        (set `MovementComponent.Velocity` (`KismetMathLibrary.ClampVectorSize` (`KismetMathLibrary.VLerp` (`MovementComponent.Velocity` (`self.CharacterMovement`)) (`KismetMathLibrary.MirrorVectorByNormal` (`MovementComponent.Velocity` (`self.CharacterMovement`)) (`KismetMathLibrary.GetDirectionUnitVector` _returnvalue_2 _returnvalue)) (`KismetMathLibrary.FClamp` (* (- _returnvalue_5 _maxdistance) 0.01) 0.0 50.0)) 0.0 1000.0) (`self.CharacterMovement`))
        (bind _sweephitresult (`self.K2_AddActorWorldOffset` (* (`KismetMathLibrary.GetDirectionUnitVector` _returnvalue _returnvalue_2) (- _returnvalue_5 _maxdistance)) true))
        (set `self.Blocked` (`GameplayStatics.BreakHitResult` _sweephitresult))
        (else
          (set `self.Blocked` false :!label _label_2)))
      (else
        (goto _label_2)))
    (elif (`self.Priority`)
      (goto _label_2)
      (else
        (goto _label)))))

(fn `UserConstructionScript`)