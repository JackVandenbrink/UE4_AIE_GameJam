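; Player controller for a two-player, side-view game in which both characters are tethered by a rope and driven from one controller.
; On start it adds HUD widgets, spawns both JackCharacters at the checkpoint or spawn point, and links them with a cable sized from DesignerVariables.
; An orthographic camera follows their midpoint, zooming with separation.
; Movement is gated by rope limits; death locks both characters, then retries through GameJamInstance, alongside retry and level-complete hotkeys.
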(event `self.ReceiveBeginPlay`
  (`self.Init`))

(event `self.ReceiveTick`
  (params (DeltaSeconds :type "Float (single-precision)"))
  (`self.CameraMovement`))

(event `InputAxis|P1_Move`
  (params (AxisValue :type "Float (single-precision)"))
  (bind _playerone (`self.PlayerOne`))
  (if (`self.MoveIgnored`)
    _
    (elif (== (`KismetMathLibrary.FTrunc` AxisValue) 0)
      _
      (elif (`/Game/Jack/Blueprints/JackCharacter.CanIMoveAway` _playerone)
        (`Pawn.AddMovementInput` _playerone (`self.MoveRight`) AxisValue false :!label _label)
        (else
          (bind _return (`self.WillMoveCloser` _playerone AxisValue))
          (if _return
            (goto _label)))))))

(event `InputAxis|P2_Move`
  (params (AxisValue :type "Float (single-precision)"))
  (bind _playertwo (`self.PlayerTwo`))
  (if (`self.MoveIgnored`)
    _
    (elif (== (`KismetMathLibrary.FTrunc` AxisValue) 0)
      _
      (elif (`/Game/Jack/Blueprints/JackCharacter.CanIMoveAway` _playertwo)
        (`Pawn.AddMovementInput` _playertwo (`self.MoveRight`) AxisValue false :!label _label_2)
        (else
          (bind _return (`self.WillMoveCloser` _playertwo AxisValue))
          (if _return
            (goto _label_2)))))))

(event `InputAction|P1_Jump`
  (params (Key :type "Key Structure" :default "AnyKey"))
  (bind _playerone (`self.PlayerOne`))
  (:`Pressed`
    (if (not (`self.MoveIgnored`))
      (`/Game/Jack/Blueprints/JackCharacter.Jumped` _playerone (`Character.CanJump` _playerone))
      (`Character.Jump` _playerone)))
  (:`Released`
    (`Character.StopJumping` _playerone)))

(event `InputAction|P2_Jump`
  (params (Key :type "Key Structure" :default "AnyKey"))
  (bind _playertwo (`self.PlayerTwo`))
  (:`Pressed`
    (if (not (`self.MoveIgnored`))
      (`/Game/Jack/Blueprints/JackCharacter.Jumped` _playertwo (`Character.CanJump` _playertwo))
      (`Character.Jump` _playertwo)))
  (:`Released`
    (`Character.StopJumping` _playertwo)))

(event `Key|G`
  (params (Key :type "Key Structure" :default "AnyKey"))
  (:`Pressed`
    (bind _asgame_jam_instance (cast `/Game/GameJamInstance` (`GameplayStatics.GetGameInstance`)))
    (`/Game/GameJamInstance.LevelComplete` _asgame_jam_instance)))

(event `Key|T`
  (params (Key :type "Key Structure" :default "AnyKey"))
  (bind _playerone (`self.PlayerOne`))
  (:`Pressed`
    (`/Game/Jack/Blueprints/JackCharacter.Lock` _playerone true :!label _label_3)
    (`/Game/Jack/Blueprints/JackCharacter.Lock` (`self.PlayerTwo`) true)
    (`/Game/Jack/Blueprints/JackCharacter.Died` _playerone)
    (`/Game/Jack/Blueprints/JackCharacter.Died` (`self.PlayerTwo`))
    (`/Game/Jack/Blueprints/JackCharacter.ChangeAnimation` (`self.PlayerOne`) "NewEnumerator5")
    (bind _time (`/Game/Jack/Blueprints/JackCharacter.ChangeAnimation` (`self.PlayerTwo`) "NewEnumerator5"))
    (`KismetSystemLibrary.Delay` _time)
    (bind _asgame_jam_instance (cast `/Game/GameJamInstance` (`GameplayStatics.GetGameInstance`)))
    (`/Game/GameJamInstance.Retry` _asgame_jam_instance)))

(event `KillPlayer`
  (goto _label_3))

(event `Key|R`
  (params (Key :type "Key Structure" :default "AnyKey"))
  (:`Pressed`
    (bind _asgame_jam_instance (cast `/Game/GameJamInstance` (`GameplayStatics.GetGameInstance`)))
    (`/Game/GameJamInstance.Retry` _asgame_jam_instance)))

(fn `AddRope`
  (bind _asdesigner_variables (`self.GetGameState`))
  (bind _returnvalue (`|SpawnActorFromClass` "/Script/CableComponent.CableActor" (`KismetMathLibrary.MakeTransform` (`self.K2_GetActorLocation` (`self.PlayerOne`))) "Undefined" "OverrideRootScale"))
  (bind _output_get (set `self.Cable` _returnvalue))
  (bind _cablecomponent (`CableActor.CableComponent` _output_get))
  (set `CableComponent.SolverIterations` 10 _cablecomponent)
  (set `CableComponent.CableLength` (- (`/Game/DesignerVariables.MaxRopeLength` _asdesigner_variables) 100.0) _cablecomponent)
  (`PrimitiveComponent.SetMaterial` (`CableActor.CableComponent` _output_get) 0 (`/Game/DesignerVariables.RopeMaterial` _asdesigner_variables))
  (`self.K2_AttachToActor` _output_get (`self.PlayerOne`) "None" "SnapToTarget" "KeepRelative" "KeepWorld" false)
  (`CableComponent.SetAttachEndTo` (`CableActor.CableComponent` _output_get) (`self.PlayerTwo`) "None" "None"))

(fn `AddWidgets`
  (bind _returnvalue (`GameplayStatics.GetPlayerController` 0))
  (bind _returnvalue_2 (`|CreateWidget` "/Game/Ryuto/Blueprints/Widgets/attempCounter.attempCounter_C" _returnvalue))
  (`/Game/Ryuto/Blueprints/Widgets/BaseWidget.toggle` _returnvalue_2 true)
  (bind _returnvalue_3 (`|CreateWidget` "/Game/Ryuto/Blueprints/Widgets/TimeSpent.TimeSpent_C" _returnvalue))
  (`/Game/Ryuto/Blueprints/Widgets/BaseWidget.toggle` _returnvalue_3 true)
  (bind _returnvalue_4 (`|CreateWidget` "/Game/Jack/Blueprints/Widgets/BackToMainMenu.BackToMainMenu_C" _returnvalue))
  (set `self.LevelSelectButton` _returnvalue_4)
  (`/Game/Ryuto/Blueprints/Widgets/BaseWidget.toggle` _returnvalue_4 true))

(fn `CameraMovement`
  (bind _cam (`self.Cam`))
  (bind _returnvalue (`self.K2_GetActorLocation` (`self.PlayerTwo`)))
  (bind _returnvalue_2 (`self.K2_GetActorLocation` (`self.PlayerOne`)))
  (`self.K2_SetActorLocation` _cam (`KismetMathLibrary.MakeVector` -500.0 (.y (/ (+ _returnvalue_2 _returnvalue) 2)) (.z (/ (+ _returnvalue_2 _returnvalue) 2))) false false)
  (`CameraComponent.SetOrthoWidth` (`CameraActor.CameraComponent` _cam) (`KismetMathLibrary.FClamp` (+ (`KismetMathLibrary.VSize` (- _returnvalue_2 _returnvalue)) 1000.0) 2000.0 4500.0)))

(fn `GetGameState`
  (returns (`AsDesigner Variables` :type "/Game/DesignerVariables Object Reference"))
  (bind _asdesigner_variables (cast `/Game/DesignerVariables` (`GameplayStatics.GetGameState`)))
  (return _asdesigner_variables))

(fn `GiveNames`
  (bind _asname (cast `/Game/Ryuto/Blueprints/Widgets/Name` (`WidgetComponent.GetUserWidgetObject` (`/Game/Jack/Blueprints/JackCharacter.Widget` (`self.PlayerOne`)))))
  (`/Game/Ryuto/Blueprints/Widgets/Name.setName` _asname "P1")
  (bind _asname_2 (cast `/Game/Ryuto/Blueprints/Widgets/Name` (`WidgetComponent.GetUserWidgetObject` (`/Game/Jack/Blueprints/JackCharacter.Widget` (`self.PlayerTwo`)))))
  (`/Game/Ryuto/Blueprints/Widgets/Name.setName` _asname_2 "P2"))

(fn `Init`
  (`self.AddWidgets`)
  (bind _outactors (`GameplayStatics.GetAllActorsOfClass` "/Script/Engine.CameraActor"))
  (bind _item (`KismetArrayLibrary.Array_Get` _outactors))
  (bind _output_get (set `self.Cam` _item))
  (`CameraComponent.SetProjectionMode` (`CameraActor.CameraComponent` _output_get) "Orthographic")
  (`self.SetViewTargetWithBlend` _item)
  (`self.SpawnPlayers`)
  (`self.AddRope`)
  (`self.GiveNames`)
  (`self.SetActorTickEnabled` true)
  (`WidgetBlueprintLibrary.SetInputMode_GameAndUIEx` self (`self.LevelSelectButton`) "DoNotLock" false)
  (set `self.bShowMouseCursor` true))

(fn `SpawnPlayers`
  (`|ExecutionSequence`
    (:`then_0`
      (bind _asgame_jam_instance (cast `/Game/GameJamInstance` (`GameplayStatics.GetGameInstance`)))
      (bind _outactors (`GameplayStatics.GetAllActorsOfClass` "/Game/Jack/Blueprints/CharacterSpawnPoint.CharacterSpawnPoint_C"))
      (bind _returnvalue (select `bool` (`/Game/GameJamInstance.hasActiveCheckPoint` _asgame_jam_instance) :`false` (`self.K2_GetActorLocation` (`KismetArrayLibrary.Array_Get` _outactors)) :`true` (`/Game/GameJamInstance.checkPointLoc` _asgame_jam_instance)))
      (bind _returnvalue_2 (`|SpawnActorFromClass` "/Game/Jack/Blueprints/JackCharacter.JackCharacter_C" (`KismetMathLibrary.MakeTransform` _returnvalue) "AlwaysSpawn" "OverrideRootScale"))
      (bind _output_get (set `self.PlayerOne` _returnvalue_2))
      (set `/Game/Jack/Blueprints/JackCharacter.Priority` true _output_get)
      (bind _returnvalue_3 (`|SpawnActorFromClass` "/Game/Jack/Blueprints/JackCharacter.JackCharacter_C" (`KismetMathLibrary.MakeTransform` _returnvalue) "AlwaysSpawn" "OverrideRootScale"))
      (bind _output_get_2 (set `self.PlayerTwo` _returnvalue_3))
      (set `/Game/Jack/Blueprints/JackCharacter.OtherChar` _output_get_2 _output_get)
      (set `/Game/Jack/Blueprints/JackCharacter.OtherChar` _output_get _output_get_2))
    (:`then_1`
      (bind _output_get_3 (set `/Game/Jack/Blueprints/JackCharacter.MaxDistance` (`/Game/DesignerVariables.MaxRopeLength` (`self.GetGameState`)) (`self.PlayerOne`)))
      (set `/Game/Jack/Blueprints/JackCharacter.MaxDistance` _output_get_3 (`self.PlayerTwo`)))))

(fn `UserConstructionScript`)

(fn `WillMoveCloser`
  (params (MovingPlayer :type "/Game/Jack/Blueprints/JackCharacter Object Reference") (Scale :type "Float (double-precision)"))
  (returns (Return :type Boolean))
  (locals (ActualDistance :type "Float (double-precision)" :default 0.0) (DistanceAfterInput :type "Float (double-precision)"))
  (bind _returnvalue (`self.K2_GetActorLocation` MovingPlayer))
  (bind _returnvalue_2 (`self.K2_GetActorLocation` (`self.PlayerTwo`)))
  (bind (_returnvalue_x _returnvalue_y) (`KismetMathLibrary.BreakVector` (- _returnvalue _returnvalue_2)))
  (bind (_returnvalue_x_2 _returnvalue_y_2) (`KismetMathLibrary.BreakVector` (- (+ _returnvalue (* (`self.MoveRight`) Scale)) _returnvalue_2)))
  (set `local.ActualDistance` _returnvalue_y)
  (set `local.DistanceAfterInput` _returnvalue_y_2)
  (return (< (`local.DistanceAfterInput`) (`local.ActualDistance`))))