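; Pressure-plate button that opens linked gates while a JackCharacter stands on it.
; When a JackCharacter enters the Box trigger, the mesh drops, an overlap counter increments and every gate in the Gate array opens.
; Each exit raises the mesh and decrements the counter, but the gates close only when the count reaches zero.
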(event `self.Box.OnComponentBeginOverlap`
  (params (OverlappedComponent :type "PrimitiveComponent Object Reference") (OtherActor :type "Actor Object Reference") (OtherComp :type "PrimitiveComponent Object Reference") (OtherBodyIndex :type Integer) (bFromSweep :type Boolean) (SweepResult :type "HitResult Structure (by ref)"))
  (cast `/Game/Jack/Blueprints/JackCharacter` OtherActor)
  (`SceneComponent.K2_SetRelativeLocation` (`self.Mesh`) (0.0 0.0 -20.0) false false)
  (`/Engine/EditorBlueprintResources/StandardMacros.IncrementInt` (`self.Overlappers`)
    (:`  `
      (for _array_element (`self.Gate`)
        (`/Game/Jack/Blueprints/Buttons/Gate.OpenGate` _array_element)))))

(event `self.Box.OnComponentEndOverlap`
  (params (OverlappedComponent :type "PrimitiveComponent Object Reference") (OtherActor :type "Actor Object Reference") (OtherComp :type "PrimitiveComponent Object Reference") (OtherBodyIndex :type Integer))
  (cast `/Game/Jack/Blueprints/JackCharacter` OtherActor)
  (`SceneComponent.K2_SetRelativeLocation` (`self.Mesh`) (0.0 0.0 0.0) false false)
  (bind _result (`/Engine/EditorBlueprintResources/StandardMacros.DecrementInt` (`self.Overlappers`))
    (:`  `
      (if (== _result 0)
        (for _array_element (`self.Gate`)
          (`/Game/Jack/Blueprints/Buttons/Gate.CloseGate` _array_element))))))

(fn `UserConstructionScript`)