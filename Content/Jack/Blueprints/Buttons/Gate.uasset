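; Gate Blueprint that swings open and closed in response to OpenGate and CloseGate events.
; A Gate timeline plays forward or in reverse, and its Alpha lerps a SpringArm's relative rotation between the closed and open rotations.
; IsOpening and IsClosing track the direction of motion and are cleared when the timeline finishes.
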(event `OpenGate`
  (set `self.IsOpening` true)
  (set `self.IsClosing` false)
  (bind (_direction _alpha) (`Timeline|Gate` :!label _label)
    (:`Update`
      (`SceneComponent.K2_SetRelativeRotation` (`self.SpringArm`) (`KismetMathLibrary.RLerp` (`self.ClosedRot`) (`self.OpenRot`) _alpha) false false))
    (:`Finished`
      (set `self.IsOpening` false)
      (set `self.IsClosing` false))))

(event `CloseGate`
  (set `self.IsOpening` false)
  (set `self.IsClosing` true)
  (goto _label :!via `Reverse`))

(fn `UserConstructionScript`)