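; Player character Blueprint for a game jam game, elastically tethered to another character (OtherChar).
; Each tick, TestSwing checks tether overstretch, forces the character into falling, mirrors velocity scaled by overflow and nudges it inward; SwingFromOther is an uncalled lerp-based variant.
; LockPos anchors the character only while walking, with Tick reapplying the saved position.
; Falling to KillZoneZ triggers Retry on the GameJamInstance.
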(event `self.ReceiveBeginPlay`
  (`self.SpawnDefaultController`)
  (bind _asgame_jam_instance (cast `/Game/GameJamInstance` (`GameplayStatics.GetGameInstance`)))
  (`KismetSystemLibrary.PrintString` (`KismetStringLibrary.Conv_IntToString` (`/Game/GameJamInstance.RetryCount` _asgame_jam_instance))))

(event `self.ReceiveTick`
  (params (DeltaSeconds :type "Float (single-precision)"))
  (`self.TestSwing`)
  (`self.KillZ`)
  (if (`self.Locked`)
    (`self.K2_SetActorLocation` (`self.Pos`))))

(fn `KillZ`
  (if (<= (.z (`self.K2_GetActorLocation`)) (`self.KillZoneZ`))
    (bind _asgame_jam_instance (cast `/Game/GameJamInstance` (`GameplayStatics.GetGameInstance`)))
    (`/Game/GameJamInstance.Retry` _asgame_jam_instance)))

(fn `LockPos`
  (params (NewLocked :type Boolean))
  (if (`CharacterMovementComponent.IsWalking` (`self.CharacterMovement`))
    (bind _output_get (set `self.Locked` NewLocked))
    (if _output_get
      (set `self.Pos` (`self.K2_GetActorLocation`)))))

(fn `SwingFromOther`
  (bind _returnvalue (`self.K2_GetActorLocation`))
  (bind _maxdistance (`self.MaxDistance`))
  (bind _returnvalue_2 (`self.K2_GetActorLocation` (`self.OtherChar`)))
  (bind _returnvalue_3 (`KismetMathLibrary.VSize` (- _returnvalue_2 _returnvalue)))
  (bind _returnvalue_4 (`KismetMathLibrary.FClamp` (* (- _returnvalue_3 _maxdistance) 0.01) 0.0 50.0))
  (if (>= _returnvalue_3 _maxdistance)
    ;[1 1 1] Force player off the ground
    (if (> _returnvalue_4 0.5)
      (`self.Jump`)
      (`CharacterMovementComponent.SetMovementMode` (`self.CharacterMovement`) "MOVE_Falling" 0))
    ;[1 1 1] Set Velocity and Force Player Pos Inwards
    (set `MovementComponent.Velocity` (`KismetMathLibrary.ClampVectorSize` (`KismetMathLibrary.VLerp` (`MovementComponent.Velocity` (`self.CharacterMovement`)) (`KismetMathLibrary.MirrorVectorByNormal` (`MovementComponent.Velocity` (`self.CharacterMovement`)) (`KismetMathLibrary.GetDirectionUnitVector` _returnvalue_2 _returnvalue)) _returnvalue_4) 0.0 10000.0) (`self.CharacterMovement`))
    (`self.K2_AddActorWorldOffset` (* (`KismetMathLibrary.GetDirectionUnitVector` _returnvalue _returnvalue_2) _returnvalue_4) true)))

(fn `TestSwing`
  (bind _returnvalue (`self.K2_GetActorLocation`))
  (bind _maxdistance (`self.MaxDistance`))
  (bind _returnvalue_2 (`self.K2_GetActorLocation` (`self.OtherChar`)))
  (bind _returnvalue_3 (`KismetMathLibrary.VSize` (- _returnvalue_2 _returnvalue)))
  (bind _returnvalue_4 (`KismetMathLibrary.FClamp` (* (- _returnvalue_3 _maxdistance) 0.01) 0.0 50.0))
  (if (> _returnvalue_3 _maxdistance)
    (set `self.Overflow` (- _returnvalue_3 _maxdistance))
    ;[1 1 1] Force player off the ground
    (if (> _returnvalue_4 0.5)
      (`self.Jump`)
      (`CharacterMovementComponent.SetMovementMode` (`self.CharacterMovement`) "MOVE_Falling" 0)
      ;[1 1 1] Set Velocity and Force Player Pos Inwards
      (set `MovementComponent.Velocity` (`KismetMathLibrary.ClampVectorSize` (* (`KismetMathLibrary.Normal` (`KismetMathLibrary.MirrorVectorByNormal` (`MovementComponent.Velocity` (`self.CharacterMovement`)) (`KismetMathLibrary.GetDirectionUnitVector` _returnvalue_2 _returnvalue))) (`self.Overflow`)) 0.0 10000.0) (`self.CharacterMovement`))
      (`self.K2_AddActorWorldOffset` (* (`KismetMathLibrary.GetDirectionUnitVector` _returnvalue _returnvalue_2) _returnvalue_4) true))))

(fn `UserConstructionScript`)