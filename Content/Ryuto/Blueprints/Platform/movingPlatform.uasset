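; Moving platform actor that travels along the Y or Z axis at a set speed, either continuously or only while its button-pressed flag is set.
; On BeginPlay it turns per-side travel distances into world limits around its start position.
; Each tick it offsets its location by a direction enum, then reverses direction past those limits.
; Overlapping a StaticPlatform also flips it between left and right.
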(event `self.ReceiveBeginPlay`
  (`self.Init`))

(event `self.ReceiveActorBeginOverlap`
  (params (OtherActor :type "Actor Object Reference"))
  (cast `/Game/Ryuto/Blueprints/Platform/StaticPlatform` OtherActor)
  (`self.changeDir`))

(event `self.ReceiveTick`
  (params (DeltaSeconds :type "Float (single-precision)"))
  (bind _speed (`self.Speed`))
  (if (`self.moveViaButton`)
    (`self.ButtonMove` DeltaSeconds _speed (`self.buttonPressed`))
    (else
      (`self.move` DeltaSeconds _speed))))

(fn `ButtonMove`
  (params (deltatime :type "Float (double-precision)") (speed :type "Float (double-precision)") (pressed :type Boolean))
  (if pressed
    (`self.K2_SetActorLocation` (+ (`self.K2_GetActorLocation`) (* (* (select `/Game/Ryuto/Blueprints/directionEnum` (`self.direction`) :`NewEnumerator0` (0.0 -1.0 0.0) :`NewEnumerator1` (0.0 1.0 0.0) :`NewEnumerator3` (0.0 0.0 1.0) :`NewEnumerator4` (0.0 0.0 -1.0) :!type "Vector Structure") deltatime) speed)))
    (`self.checkYAxis`)
    (`self.checkZAxis`)))

(fn `changeDir`
  (if (`|EnumEquality` (`self.direction`) "NewEnumerator0")
    (set `self.direction` "NewEnumerator1")
    (else
      (set `self.direction` "NewEnumerator0"))))

(fn `checkYAxis`
  (bind _returnvalue (`KismetMathLibrary.FFloor` (.y (`self.K2_GetActorLocation`))))
  (if (< _returnvalue (`self.vecMaxLeft`))
    (set `self.direction` "NewEnumerator1")
    (elif (> _returnvalue (`self.vecMaxRight`))
      (set `self.direction` "NewEnumerator0"))))

(fn `checkZAxis`
  (bind _returnvalue (`KismetMathLibrary.FFloor` (.z (`self.K2_GetActorLocation`))))
  (if (< _returnvalue (`self.vecMaxDown`))
    (set `self.direction` "NewEnumerator3")
    (elif (> _returnvalue (`self.vecMaxUp`))
      (set `self.direction` "NewEnumerator4"))))

(fn `Init`
  (bind (_returnvalue_x _returnvalue_y _returnvalue_z) (`KismetMathLibrary.BreakVector` (`self.K2_GetActorLocation`)))
  (set `self.initSpeed` (`self.Speed`))
  (set `self.direction` (`self.initDirection`))
  (bind _output_get (set `self.startPosY` (`KismetMathLibrary.FFloor` _returnvalue_y)))
  (bind _output_get_2 (set `self.startPosZ` (`KismetMathLibrary.FFloor` _returnvalue_z)))
  (set `self.vecMaxUp` (+ _output_get_2 (`self.vecMaxUp`)))
  (set `self.vecMaxDown` (- _output_get_2 (`self.vecMaxDown`)))
  (set `self.vecMaxRight` (+ _output_get (`self.vecMaxRight`)))
  (set `self.vecMaxLeft` (- _output_get (`self.vecMaxLeft`))))

(fn `move`
  (params (deltatime :type "Float (double-precision)") (speed :type "Float (double-precision)"))
  (`self.K2_SetActorLocation` (+ (`self.K2_GetActorLocation`) (* (* (select `/Game/Ryuto/Blueprints/directionEnum` (`self.direction`) :`NewEnumerator0` (0.0 -1.0 0.0) :`NewEnumerator1` (0.0 1.0 0.0) :`NewEnumerator3` (0.0 0.0 1.0) :`NewEnumerator4` (0.0 0.0 -1.0) :!type "Vector Structure") deltatime) speed)))
  (`self.checkYAxis`)
  (`self.checkZAxis`))

(fn `UserConstructionScript`)