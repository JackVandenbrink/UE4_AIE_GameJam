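; Pressure-plate button that switches its assigned moving platforms on while a JackCharacter stands on it.
; Box overlap lowers the mesh, increments an overlap count and sets ButtonPressed on every entry in the Platform array.
; Leaving raises the mesh immediately, even if other overlaps remain, and decrements the count.
; The platforms' ButtonPressed flags clear only when that count reaches zero.
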(event `self.Box.OnComponentBeginOverlap`
  (params (OverlappedComponent :type "PrimitiveComponent Object Reference") (OtherActor :type "Actor Object Reference") (OtherComp :type "PrimitiveComponent Object Reference") (OtherBodyIndex :type Integer) (bFromSweep :type Boolean) (SweepResult :type "HitResult Structure (by ref)"))
  (cast `/Game/Jack/Blueprints/JackCharacter` OtherActor)
  (`SceneComponent.K2_SetRelativeLocation` (`self.Mesh`) (0.0 0.0 -10.0) false false)
  (`/Engine/EditorBlueprintResources/StandardMacros.IncrementInt` (`self.numOfOverlap`)
    (:`  `
      (for _array_element (`self.Platform`)
        (set `/Game/Ryuto/Blueprints/Platform/movingPlatform.buttonPressed` true _array_element)))))

(event `self.Box.OnComponentEndOverlap`
  (params (OverlappedComponent :type "PrimitiveComponent Object Reference") (OtherActor :type "Actor Object Reference") (OtherComp :type "PrimitiveComponent Object Reference") (OtherBodyIndex :type Integer))
  (bind _numofoverlap (`self.numOfOverlap`))
  (cast `/Game/Jack/Blueprints/JackCharacter` OtherActor)
  (`SceneComponent.K2_SetRelativeLocation` (`self.Mesh`) (0.0 0.0 0.0) false false)
  (`/Engine/EditorBlueprintResources/StandardMacros.DecrementInt` _numofoverlap
    (:`  `
      (if (== _numofoverlap 0)
        (for _array_element (`self.Platform`)
          (set `/Game/Ryuto/Blueprints/Platform/movingPlatform.buttonPressed` false _array_element))))))

(fn `UserConstructionScript`)